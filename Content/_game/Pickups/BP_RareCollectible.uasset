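; BP_RareCollectible is a rare pickup that the player collects by overlapping its box.
; When player 0's pawn enters the box, it adds a fixed amount to RareCount on the BallPlayerState.
; It then plays a sound and spawns a particle system at its location before destroying itself.
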(event `self.Box.OnComponentBeginOverlap`
  (params (OverlappedComponent :type "PrimitiveComponent Object Reference") (OtherActor :type "Actor Object Reference") (OtherComp :type "PrimitiveComponent Object Reference") (OtherBodyIndex :type Integer) (bFromSweep :type Boolean) (SweepResult :type "HitResult Structure (by ref)"))
  (if (== OtherActor (`GameplayStatics.GetPlayerPawn` 0))
    (bind _asball_player_state (cast `/Game/_game/BallGame/BallPlayerState` (`GameplayStatics.GetPlayerState` 0)))
    (set `/Game/_game/BallGame/BallPlayerState.RareCount` (+ (`/Game/_game/BallGame/BallPlayerState.RareCount` _asball_player_state) 4) _asball_player_state)
    (`GameplayStatics.PlaySoundAtLocation` (`self.Sound`) (`self.K2_GetActorLocation`) (struct) 1.0 1.0 0.0 null null null null)
    (`NiagaraFunctionLibrary.SpawnSystemAtLocation` (`self.System Template`) (`self.K2_GetActorLocation`))
    (`self.K2_DestroyActor`)))

(fn `UserConstructionScript`)